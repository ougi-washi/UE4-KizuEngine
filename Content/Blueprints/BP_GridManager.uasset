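; BP_GridManager builds a three-dimensional grid of BP_GridSlot actors.
; Its construction script calls InitializeGrid, which clears AllSlots and runs nested loops over XCount, YCount and ZCount.
; Each cell adds a child actor component at evenly spaced relative offsets, sets its class to BP_GridSlot and stores the spawned slot in AllSlots.
; The event graph holds no active logic.
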(fn `InitializeGrid`
  (locals (X_Current :type Integer) (Y_Current :type Integer) (Z_Current :type Integer))
  (`KismetArrayLibrary.Array_Clear` (`self.AllSlots`))
  (for _index (range 1 (+ (`self.X_Count`) 1))
    (set `local.X_Current` _index)
    (for _index_2 (range 1 (+ (`self.Y_Count`) 1))
      (set `local.Y_Current` _index_2)
      (for _index_3 (range 1 (+ (`self.Z_Count`) 1))
        (set `local.Z_Current` _index_3)
        (bind _returnvalue (`AddComponent|NODE_AddChildActorComponent-0` :`RelativeTransform` (`KismetMathLibrary.MakeTransform` (`KismetMathLibrary.MakeVector` (* (`local.X_Current`) 200.0) (* (`local.Y_Current`) 200.0) (* (`local.Z_Current`) 200.0)))))
        (`ChildActorComponent.SetChildActorClass` _returnvalue "/Game/Blueprints/BP_GridSlot.BP_GridSlot_C")
        (bind _asbp_grid_slot (cast `/Game/Blueprints/BP_GridSlot` (`ChildActorComponent.ChildActor` _returnvalue)))
        (`KismetArrayLibrary.Array_Add` (`self.AllSlots`) _asbp_grid_slot)))))

(fn `UserConstructionScript`
  (`self.InitializeGrid`))
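; BP_BLOCK is a block actor that moves along a scripted path once, starting at BeginPlay.
; BeginPlay chains MoveObject calls one second apart, stepping along Y, then X, then up and back down, then back along X, without undoing the Y offset.
; MoveObject offsets the current location into a target, then a Timeline drives a swept SetActorLocation lerp from the live location, not a stored start point.
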(event `self.ReceiveBeginPlay`
  (`self.MoveObject` (0.0 200.0 0.0))
  (`KismetSystemLibrary.Delay` 1.0)
  (`self.MoveObject` (0.0 200.0 0.0))
  (`KismetSystemLibrary.Delay` 1.0)
  (`self.MoveObject` (-200.0 -0.0 0.0))
  (`KismetSystemLibrary.Delay` 1.0)
  (`self.MoveObject` (-200.0 0.0 0.0))
  (`KismetSystemLibrary.Delay` 1.0)
  (`self.MoveObject` (0.0 -0.0 200.0))
  (`KismetSystemLibrary.Delay` 1.0)
  (`self.MoveObject` (0.0 0.0 200.0))
  (`KismetSystemLibrary.Delay` 1.0)
  (`self.MoveObject` (0.0 -0.0 -200.0))
  (`KismetSystemLibrary.Delay` 1.0)
  (`self.MoveObject` (0.0 0.0 -200.0))
  (`KismetSystemLibrary.Delay` 1.0)
  (`self.MoveObject` (200.0 -0.0 0.0))
  (`KismetSystemLibrary.Delay` 1.0)
  (`self.MoveObject` (200.0 0.0 0.0))
  (`KismetSystemLibrary.Delay` 1.0))

(event `self.ReceiveTick`
  (params (DeltaSeconds :type "Float (single-precision)")))

(event `MoveObject`
  (params (MoveValue :type "Vector Structure"))
  (set `self.TargetValue` (+ (`self.K2_GetActorLocation`) MoveValue))
  (bind (_direction _newtrack_1) (`Timeline|Timeline_0` :!via `PlayFromStart`)
    (:`Update`
      (`self.K2_SetActorLocation` (`KismetMathLibrary.VLerp` (`self.K2_GetActorLocation`) (`self.TargetValue`) _newtrack_1) true))))

(fn `UserConstructionScript`)
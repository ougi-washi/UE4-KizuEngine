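; BP_Point1 is an actor that prints the look-at rotation from itself toward a BP_Point2 actor on screen.
; On BeginPlay it caches the first BP_Point2 found in the level.
; Each Tick it computes FindLookAtRotation between the two locations and shows it as short-lived red debug text, without rotating either actor.
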(event `self.ReceiveBeginPlay`
  (bind _outactors (`GameplayStatics.GetAllActorsOfClass` "/Game/Blueprints/BP_Point2.BP_Point2_C"))
  (set `self.Point2` (`|GetArrayItem` _outactors)))

(event `self.ReceiveTick`
  (params (DeltaSeconds :type "Float (single-precision)"))
  (`KismetSystemLibrary.PrintString` (`KismetStringLibrary.Concat_StrStr` "Rotation " (`KismetStringLibrary.Conv_RotatorToString` (`KismetMathLibrary.FindLookAtRotation` (`self.K2_GetActorLocation`) (`self.K2_GetActorLocation` (`self.Point2`))))) true true (struct :`R` 1.0 :`B` 0.007073 :`A` 1.0) 0.1))

(fn `UserConstructionScript`)